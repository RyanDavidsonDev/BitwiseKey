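; Player character Blueprint that handles death on hazard contact and toggles the pause menu.
; Overlapping an actor tagged KillPlayer calls CallDOnReset on the CustomGameMode.
; The IA_Pause input creates and caches the pause menu widget on first use, then calls its TogglePause, with a debug print on later presses.
; Older inline pause, resume and game-mode reset nodes remain disconnected and never run.
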(event `self.ReceiveBeginPlay`)

(event `self.ReceiveActorBeginOverlap`
  (params (OtherActor :type "Actor Object Reference"))
  (if (`self.ActorHasTag` OtherActor "KillPlayer")
    (`CustomGameMode.D_OnReset` (cast `CustomGameMode` (`GameplayStatics.GetGameMode`) :!pure true))))

(event `EnhancedInput|/Game/UserInput/IA_Pause`
  (params (ActionValue :type Boolean) (ElapsedSeconds :type "Float (double-precision)") (TriggeredSeconds :type "Float (double-precision)") (InputAction :type "InputAction Object Reference" :default "/Game/UserInput/IA_Pause.IA_Pause"))
  (:`Started`
    (`/Engine/EditorBlueprintResources/StandardMacros.IsValid` (`self.PauseMenuReference`)
      (:`Is Valid`
        (`KismetSystemLibrary.PrintString` "paused"))
      (:`Is Not Valid`
        (bind _returnvalue (`|CreateWidget` "/Game/UI/PauseMenuWidget.PauseMenuWidget_C"))
        (bind _output_get (set `self.PauseMenuReference` _returnvalue))))
    (`/Game/UI/PauseMenuWidget.TogglePause` _output_get)))

(fn `UserConstructionScript`)