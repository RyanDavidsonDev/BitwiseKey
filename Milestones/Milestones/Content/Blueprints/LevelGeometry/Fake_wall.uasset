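; Fake wall level geometry that is solid until an X-ray pickup is collected, then becomes passable.
; On BeginPlay it binds to CustomGameMode's X-ray collected and reset delegates and sets its solid, particle-free default state.
; Collection activates the particles and disables mesh collision, while reset restores the default.
; Material swaps to and from a translucent hex look are present but disconnected.
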(event `self.ReceiveBeginPlay`
  (bind _ascustom_game_mode (cast `CustomGameMode` (`GameplayStatics.GetGameMode`) :!pure true))
  (add `CustomGameMode.D_OnReset` _ascustom_game_mode (delegate `ResetWall`))
  (add `CustomGameMode.OnCollectedXray` _ascustom_game_mode (delegate `XrayCollected`))
  ;[1 1 1] Initialize the actor - set values to no collison and no particles
  (`ActorComponent.Deactivate` (`self.particles`) :!label _label)
  (`PrimitiveComponent.SetCollisionEnabled` (`self.StaticMeshComponent`) "QueryAndPhysics"))

(event `ResetWall`
  (goto _label))

(event `XrayCollected`
  ;[1 1 1] enable all the new stuff when the delegate gets activated
  (`ActorComponent.Activate` (`self.particles`) false)
  (`PrimitiveComponent.SetCollisionEnabled` (`self.StaticMeshComponent`) "NoCollision")
  (`KismetSystemLibrary.PrintString` "delegate received"))

(fn `UserConstructionScript`)